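; Fish pawn for a fishing game that reacts to the player's Fisher pawn.
; Each tick it turns, yaw only, to face its velocity.
; Escape waits a second, then uses AI navigation to swim to a random point around the cast point.
; Pull steps it toward the player at a fixed height, despite a comment saying "swim away"; Move is an empty stub.
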(event Custom|Move_1)

(event Custom|Escape_1
  (bind _asfisher (Utilities|Casting|CastToFisher (Game|Player|GetPlayerPawn 0)))
  (Utilities|FlowControl|Delay 1.0)
  (AI|Navigation|SimpleMovetoLocation (Pawn|GetController) (Math|Vector|MakeVector (.x (.RandomLocation (Class|NavigationSystemV1|GetRandomPointinNavigableRadius (Variables|/Script/FishingMiniGame.Fisher|GetCastPoint _asfisher) 1e+03 0 "/Script/AIModule.NavFilter_AIControllerDefault"))) (.y (.RandomLocation (Class|NavigationSystemV1|GetRandomPointinNavigableRadius (Variables|/Script/FishingMiniGame.Fisher|GetCastPoint _asfisher) 1e+03 0 "/Script/AIModule.NavFilter_AIControllerDefault"))) (.z (Transformation|GetActorLocation)))))

(event Custom|Pull_1
  (Utilities|Casting|CastToFisher (Game|Player|GetPlayerPawn 0))
  (Transformation|SetActorLocation (Math|Vector|MakeVector (.x (+ (Transformation|GetActorLocation) (* (Math|Vector|Normalize (- (Transformation|GetActorLocation (stale Custom|Escape_1 _asfisher)) (Transformation|GetActorLocation))) 25))) (.y (+ (Transformation|GetActorLocation) (* (Math|Vector|Normalize (- (Transformation|GetActorLocation (stale Custom|Escape_1 _asfisher)) (Transformation|GetActorLocation))) 25))) 6e+01) false false))

(event EventTick
  (params (DeltaSeconds :type Float%20%28single-precision%29))
  (|Facewheremoving))

(fn ConstructionScript)