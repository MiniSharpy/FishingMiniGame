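; Fishing player Blueprint that runs a cast, bite and reel loop through an Idle, Casting, Casted and Reeling state machine on one input.
; A world-space arrow follows the mouse, and a smoothstepped ping-pong timer sets cast strength, placing the bait along it.
; After a bite event, presses impulse the attached fish toward the player while Tick derives the reel value from fish velocity.
; Success handling is empty, and debug drawing remains active.
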(event Custom|OnFailure
  (CallFunction|ResetFishing))

(event Custom|OnSuccess)

(event Custom|OnFishBite
  (Variables|Default|SetFishBit true))

(event Custom|SetWidgetLengthInEditor
  (CallFunction|SetWidgetLength))

(event Custom|SetAttachedFish
  (params (Fish :type BP%20Fish%20Old%20Object%20Reference))
  (Variables|Default|SetAttachedFish Fish))

(event EventBeginPlay
  (Variables|Default|SetWidgetStartingRotation (Transformation|GetWorldRotation (Variables|Default|GetCastDirectionWidget)))
  (CallFunction|SetWidgetLength)
  (bind _returnvalue (UserInterface|CreateWidget "/Game/Interface/Widget_Reel.Widget_Reel_C"))
  (bind _output_get (Variables|Default|SetReelingWidget _returnvalue))
  (UserInterface|Viewport|AddtoViewport _output_get 0)
  (Widget|SetVisibility (Variables|Default|GetReelingWidget) "Hidden"))

(event EventTick
  (params (DeltaSeconds :type Float%20%28single-precision%29))
  (bind _castdirectionwidget (Variables|Default|GetCastDirectionWidget))
  (bind _widgetstartingrotation (Variables|Default|GetWidgetStartingRotation))
  (bind _returnvalue (Transformation|GetWorldLocation _castdirectionwidget))
  (Utilities|FlowControl|Sequence ; Makes things more readable
    (:then_0
      ;[1 1 1] Setting Widget Rotation
      (bind _asplayer_controller (Utilities|Casting|CastToPlayerController (Pawn|GetController)))
      (Variables|/Script/Engine.PlayerController|SetbShowMouseCursor _asplayer_controller true)
      (if (.HitResult_Blocking_Hit (|GetMouseWorldPosition _asplayer_controller)) ; So if false arrow rotation doesn't reset if mouse is outside of water.
        (Variables|Default|SetMouseDirection (Math|Vector2D|MakeVector2D (.x (Math|Vector|Normalize (Math|Vector|MakeVector (- (.HitResult_Location_X (|GetMouseWorldPosition _asplayer_controller)) (.x _returnvalue)) (- (.HitResult_Location_Y (|GetMouseWorldPosition _asplayer_controller)) (.y _returnvalue)) 0.0))) (.y (Math|Vector|Normalize (Math|Vector|MakeVector (- (.HitResult_Location_X (|GetMouseWorldPosition _asplayer_controller)) (.x _returnvalue)) (- (.HitResult_Location_Y (|GetMouseWorldPosition _asplayer_controller)) (.y _returnvalue)) 0.0)))))
        (Transformation|SetWorldRotation (Variables|Default|GetCastDirectionWidget) (Math|Rotator|MakeRotator (.roll _widgetstartingrotation) (.pitch _widgetstartingrotation) (Class|KismetMathLibrary|DegAtan2 (.y (Variables|Default|GetMouseDirection)) (.x (Variables|Default|GetMouseDirection)))) false false)))
    (:then_1
      (switch Utilities|FlowControl|Switch|SwitchonEPlayerState (Variables|Default|GetCurrentPlayerState)
        (:NewEnumerator0
          ;[1 1 1] Setting Widget Progress
          (Variables|Default|SetTime (+ DeltaSeconds (Variables|Default|GetTime)))
          (if (>= (* (|((t*t)*(3-(2*t))) (/ (Variables|Default|GetTime) (Variables|Default|GetCastDuration))) 2.0) 1.0)
            (Variables|Default|SetCastStrength (- 1.0 (- (* (|((t*t)*(3-(2*t))) (/ (Variables|Default|GetTime) (Variables|Default|GetCastDuration))) 2.0) 1.0)))
            (else
              (Variables|Default|SetCastStrength (* (|((t*t)*(3-(2*t))) (/ (Variables|Default|GetTime) (Variables|Default|GetCastDuration))) 2.0))))
          (if (>= (Variables|Default|GetTime) (Variables|Default|GetCastDuration))
            (Variables|Default|SetTime 0.0)))
        (:NewEnumerator1
          (Variables|Default|SetReelingWidgetValue (.y (Math|Vector|Normalize (Transformation|GetVelocity (Variables|Default|GetAttachedFish))))))))
    (:then_2
      (Rendering|Debug|DrawDebugSphere (Variables|Default|GetBait%20Position) 2e+01 12 "(R=1.000000,G=1.000000,B=1.000000,A=1.000000)" 0.0)
      (Development|PrintString (Utilities|String|EnumtoString (Variables|Default|GetCurrentPlayerState)) true true "(R=0.000000,G=0.660000,B=1.000000,A=1.000000)" 0.0))))

(event Input|ActionEvents|InputActionCast/Reel
  (params (Key :type Key%20Structure))
  (:Pressed
    (switch Utilities|FlowControl|Switch|SwitchonEPlayerState (Variables|Default|GetCurrentPlayerState)
      (:NewEnumerator2
        (Variables|Default|SetCurrentPlayerState "NewEnumerator0") ; Begin casting
      )
      (:NewEnumerator0
        ;[1 1 1] Finished Casting, begin wait for bite.
        (bind _arrowendpoint (CallFunction|GetArrowEndPoint (Variables|Default|GetCastStrength)))
        (Variables|Default|SetBait%20Position _arrowendpoint)
        (Development|SetHiddeninGame (Variables|Default|GetCastDirectionWidget) true false)
        (Variables|Default|SetCurrentPlayerState "NewEnumerator3"))
      (:NewEnumerator3
        (if (Variables|Default|GetFishBit)
          ;[1 1 1] Begin reeling minigame
          (Variables|Default|SetCurrentPlayerState "NewEnumerator1")
          ;;[1 1 1] Set somewhere to prevent new fish getting caught in the middle of a reel
          (Variables|Default|SetBait%20Position (Transformation|GetActorLocation))
          (Widget|SetVisibility (Variables|Default|GetReelingWidget) "HitTestInvisible")
          (else
            (CallFunction|ResetFishing))))
      (:NewEnumerator1
        (Physics|AddImpulse (Variables|/Game/Blueprints/BP_FishOld.BP_FishOld_C|GetStaticMesh (Variables|Default|GetAttachedFish)) (* (Math|Vector|Normalize (- (Transformation|GetActorLocation) (Transformation|GetActorLocation (Variables|Default|GetAttachedFish)))) 100) "None" true) ; Clear force?
        (Development|PrintString "Impulse")))))

(fn ConstructionScript)

(fn GetArrowEndPoint
  (params (CastStrength :type Float%20%28single-precision%29))
  (return (+ (Transformation|GetWorldLocation (Variables|Default|GetCastDirectionWidget)) (Math|Conversions|ToVector(Vector2D) (* (Variables|Default|GetMouseDirection) (* (* (Variables|Default|GetArrowLength) 2.0) CastStrength))))))

(fn ResetFishing
  (Variables|Default|SetFishBit false)
  (Development|SetHiddeninGame (Variables|Default|GetCastDirectionWidget) false false)
  (Variables|Default|SetCurrentPlayerState "NewEnumerator2")
  ;[1 1 1] Resetting cast
  (Variables|Default|SetCastStrength 0.0)
  (Variables|Default|SetTime 0.0)
  (Widget|SetVisibility (Variables|Default|GetReelingWidget) "Hidden"))

(fn SetWidgetLength
  ;[1 1 1] Setting Scale to be 1UE Unit(1cm), this is so length can then be equal to arrow length
  (Transformation|SetRelativeScale3D (Variables|Default|GetCastDirectionWidget) (/ (Variables|/Script/Engine.SceneComponent|GetRelativeScale3D (Variables|Default|GetCastDirectionWidget)) (.x (.BoxExtent (Collision|GetComponentBounds (Variables|Default|GetCastDirectionWidget))))))
  ;[1 1 1] Setting scale to be arrow length
  (Transformation|SetRelativeScale3D (Variables|Default|GetCastDirectionWidget) (* (Variables|/Script/Engine.SceneComponent|GetRelativeScale3D (Variables|Default|GetCastDirectionWidget)) (Variables|Default|GetArrowLength))))